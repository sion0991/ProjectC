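; BP_Cristal is a crystal that cracks and shatters shortly after the player touches it.
; A Box overlap with C_Player waits briefly, then calls BreakCristal.
; The BreakValue timeline drives opacity, crack intensity and crack normal strength on the mesh's dynamic material.
; When the timeline finishes, the actor is destroyed and BP_BreakCristal spawns at its transform.
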(event OnComponentBeginOverlap(Box)
  (params (OverlappedComponent :type Primitive%20Component%20Object%20Reference) (OtherActor :type Actor%20Object%20Reference) (OtherComp :type Primitive%20Component%20Object%20Reference) (OtherBodyIndex :type Integer) (bFromSweep :type Boolean) (SweepResult :type Hit%20Result%20Structure%20%28by%20ref%29))
  (Utilities|Casting|CastToC_Player OtherActor)
  (Utilities|FlowControl|Delay 1.0)
  (CallFunction|BreakCristal))

(event Custom|BreakCristal
  (bind _staticmesh (Variables|Default|GetStaticMesh))
  (bind _새_트랙_0 (Timeline|BreakValue PlayFromStart)
    (:Update
      (Rendering|Material|SetScalarParameterValueonMaterials _staticmesh "Opacity" (* _새_트랙_0 0.15))
      (Rendering|Material|SetScalarParameterValueonMaterials _staticmesh "Cracks_Intensity" (* _새_트랙_0 1.0))
      (Rendering|Material|SetScalarParameterValueonMaterials _staticmesh "Cracks_Normal_Intensity" (* _새_트랙_0 2e+01)))
    (:Finished
      (Actor|DestroyActor)
      (Game|SpawnActorfromClass "/Game/BP_BreakCristal.BP_BreakCristal_C" (Transformation|GetActorTransform) "AlwaysSpawn" "MultiplyWithRoot" 0 0))))

(event EventBeginPlay
  (bind _returnvalue (Rendering|Material|CreateDynamicMaterialInstance (Variables|Default|GetStaticMesh) 0 0 "None" :!class /Script/Engine.PrimitiveComponent))
  (Variables|Default|SetBrakeMat _returnvalue))

(event Collision|EventActorBeginOverlap
  (params (OtherActor :type Actor%20Object%20Reference)))

(event EventTick
  (params (DeltaSeconds :type Float%20%28single-precision%29)))

(fn ConstructionScript)