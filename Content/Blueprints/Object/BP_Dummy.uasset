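; BP_Dummy is a dummy actor that can be claimed for use, apparently as a training spot.
; The construction script sets TrainingPos to a point a short distance in front of the actor along its forward vector.
; UseDummy acts as a claim check, setting IsUsed and returning true if free, or false if already taken; nothing here resets the flag.
; The event graph holds only empty default events.
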(event EventBeginPlay)

(event Collision|EventActorBeginOverlap
  (params (OtherActor :type Actor%20Object%20Reference)))

(event EventTick
  (params (DeltaSeconds :type Float%20%28single-precision%29)))

(fn ConstructionScript
  (Variables|Default|SetTrainingPos (+ (Transformation|GetActorLocation) (* (Transformation|GetActorForwardVector) 1.5e+02))))

(fn UseDummy
  (if (Variables|Default|GetIsUsed)
    (return false)
    (else
      (Variables|Default|SetIsUsed true)
      (return true))))