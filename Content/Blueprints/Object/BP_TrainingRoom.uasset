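; Training room actor that hands out close-quarters dummies and archery targets as practice spots.
; On BeginPlay, SetTrainPos caches world transforms from both instanced static mesh components with usable flags, using the dummy count for both.
; UseDummy returns the first free spot of the requested type and marks it taken; nothing here frees it.
; Helpers that generate wall, dummy and target instances are disconnected from the construction script.
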(event EventBeginPlay
  (|SetTrainPos))

(fn ConstructionScript)

(fn UseDummy
  (params (IsCloseQuater :type Boolean))
  (bind _dummies (Variables|Default|GetDummies))
  (bind _archerytagets (Variables|Default|GetArcheryTagets))
  (if IsCloseQuater
    (for (_array_element _array_index) _dummies
      (if (.IsUsable (Utilities|Struct|BreakF_FacilityPoint _array_element))
        (Utilities|Array|SetArrayElem _dummies _array_index (Utilities|Struct|MakeF_FacilityPoint (.Tranform (Utilities|Struct|BreakF_FacilityPoint _array_element)) false))
        (return (.Tranform (Utilities|Struct|BreakF_FacilityPoint _array_element)) true)))
    (return "" false)
    (else
      (for (_array_element_2 _array_index_2) _archerytagets
        (if (.IsUsable (Utilities|Struct|BreakF_FacilityPoint _array_element_2))
          (Utilities|Array|SetArrayElem _archerytagets _array_index_2 (Utilities|Struct|MakeF_FacilityPoint (.Tranform (Utilities|Struct|BreakF_FacilityPoint _array_element_2)) false))
          (return (.Tranform (Utilities|Struct|BreakF_FacilityPoint _array_element_2)) true)))
      (return "" false))))