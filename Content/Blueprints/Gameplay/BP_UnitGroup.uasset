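; BP_UnitGroup manages a group of troops as one unit for movement and line formation.
; AddTroop registers unique members, and GroupMove writes one shared TargetLocation to each troop's Blackboard.
; LocationSetting spaces two or more troops evenly across Width, centered on the group actor along world Y, placing them through a DoOnce.
; SelectGroup and CalculationDir are unfinished stubs, and LocationSetting still prints debug output.
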(fn ConstructionScript)

(fn GroupMove
  (params (Location :type Vector))
  (for _array_element (Variables|Default|GetTroops)
    (AI|Components|Blackboard|SetValueasVector (AI|GetBlackboard _array_element) (Utilities|Name|MakeLiteralName "TargetLocation") Location)))

(fn CalculationDir)

(fn SelectGroup
  (Utilities|Array|ForEachLoopwithBreak (Variables|Default|GetTroops)))

(fn AddTroop
  (params (Troop :type BP%20NPC%20Object%20Reference%20%28by%20ref%29))
  (Utilities|Array|AddUnique (Variables|Default|GetTroops) Troop))

(fn LocationSetting
  (bind _width (Variables|Default|GetWidth))
  (bind _troops (Variables|Default|GetTroops))
  (bind _returnvalue (Utilities|Array|Length _troops))
  (bind _returnvalue_2 (- _returnvalue 1))
  (if (not (< (Utilities|Array|Length (Variables|Default|GetTroops)) 2))
    (LocalVariables|SetInterval (/ _width (Math|Integer|Clamp(Integer) _returnvalue_2 1 100)))
    (LocalVariables|SetStartX (/ _width -2))
    (for _index (range 0 _returnvalue_2)
      (Utilities|Array|AddUnique (Variables|Default|GetPos) (+ (* _index (LocalVariables|GetInterval)) (LocalVariables|GetStartX)))
      (Development|PrintString (Utilities|String|ToString(Float) (LocalVariables|GetStartX))))
    (Utilities|FlowControl|DoOnce false
      (:Completed
        (for (_array_element _array_index) (Variables|Default|GetTroops)
          (Transformation|SetActorLocation _array_element (+ (Transformation|GetActorLocation) (Math|Vector|MakeVector 0.0 (Utilities|Array|Get(acopy) (Variables|Default|GetPos) _array_index) 0.0)) false false))))))