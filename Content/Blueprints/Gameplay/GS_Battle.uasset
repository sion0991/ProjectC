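; GS_Battle tracks the live mob count in a battle and ends it with rewards when no mobs remain.
; BeginPlay counts all C_Mob actors, and CountNumOfMob adjusts that total by a given amount, calling EndGame below one.
; EndGame rolls each RewardData entry against its paired percentage, collects successes in SuccessReward, then shows the WBP_Reward widget.
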(event Custom|EndGame
  (for _array_element (Variables|Default|GetRewardData)
    (for (_array_element_2 _array_index) (.rewardindex _array_element)
      (if (<= (Math|Random|RandomInteger 100) (Utilities|Array|Get(acopy) (.probability _array_element) _array_index))
        (Utilities|Array|Add (Variables|Default|GetSuccessReward) _array_element_2))))
  (bind _returnvalue (UserInterface|CreateWidget "/Game/Blueprints/UI/WBP_Reward.WBP_Reward_C"))
  (UserInterface|Viewport|AddtoViewport _returnvalue 0))

(event Custom|CountNumOfMob
  (params (Count :type Integer))
  (bind _output_get (Variables|Default|SetCurrentMobIndex (+ (Variables|Default|GetCurrentMobIndex) Count)))
  (if (< _output_get 1)
    (CallFunction|EndGame)))

(event EventBeginPlay
  (bind _outactors (Actor|GetAllActorsOfClass "/Game/Blueprints/Character/AI/C_Mob.C_Mob_C"))
  (Variables|Default|SetCurrentMobIndex (Utilities|Array|Length _outactors)))

(event EventTick
  (params (DeltaSeconds :type Float%20%28single-precision%29)))

(fn ConstructionScript)