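; BP_NPC is a team-1 AI character with skills, a 3D HP widget, a selection decal and weapon-specific training montages.
; When perception detects a BP_MobTest, it becomes the group's enemy if none exists; SetEnemy writes target and behavior to the blackboard.
; A behavior priority list can be reordered to switch the blackboard behavior.
; Incoming damage makes the causer run AttackToTarget on the NPC with a test gameplay effect.
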(event OnTargetPerceptionUpdated(AIPerception)
  (params (Actor :type Actor%20Object%20Reference) (Stimulus :type AI%20Stimulus%20Structure))
  (bind _asbp_mob_test (Utilities|Casting|CastToBP_MobTest Actor))
  (Utilities|IsValid (Variables|/Script/ProjectC.UnitGroup|GetEnemy (Variables|Default|GetCurrentGroup))
    (:Is%20Not%20Valid
      (Class|UnitGroup|SetEnemy (Variables|Default|GetCurrentGroup) _asbp_mob_test))))

(event EventBeginPlay
  (|CallParentFunction)
  (|Init3DHPWidget)
  (CallFunction|InitializeSkill (Variables|Default|GetRow))
  (Variables|Default|SetTeamId (Utilities|Struct|MakeGenericTeamId 1)))

(event Game|Damage|EventAnyDamage
  (params (Damage :type Float%20%28single-precision%29) (DamageType :type Damage%20Type%20Object%20Reference) (InstigatedBy :type Controller%20Object%20Reference) (DamageCauser :type Actor%20Object%20Reference))
  (bind _asbp_character_base (Utilities|Casting|CastToBP_CharacterBase DamageCauser))
  (Class|RPGCharacter|AttacktoTarget _asbp_character_base self "/Game/Blueprints/AbilitySystem/GameplayEffect/BPGE_AttackTest.BPGE_AttackTest_C"))

(event EventSetEnemy
  (params (Enemy :type Actor%20Object%20Reference))
  (bind _returnvalue (AI|GetBlackboard 0))
  (AI|Components|Blackboard|SetValueasEnum _returnvalue (Utilities|Name|MakeLiteralName "Behavior") (Utilities|Enum|LiteralenumE_NPCbehavior "NewEnumerator7"))
  (AI|Components|Blackboard|SetValueasObject _returnvalue (Utilities|Name|MakeLiteralName "TargetActor") Enemy)
  (CallFunction|AddBehaviorPriority "NewEnumerator7"))

(event EventIsSelect
  (params (IsSelected :type Boolean))
  (Rendering|SetVisibility (Variables|Default|GetDecal) IsSelected false))

(fn ConstructionScript)

(fn OnActiveTraining
  (params (TargetTransform :type Transform))
  (Transformation|SetActorRotation (Math|Rotator|MakeRotator 0.0 0.0 (.yaw (Math|Rotator|FindLookatRotation (Transformation|GetActorLocation) (.location TargetTransform)))))
  (Animation|PlayAnimMontage "/Game/Mesh/Character/Player/Animation/AM_Training.AM_Training" 1.0 (Utilities|String|StringToName (Utilities|String|EnumtoString (Variables|Default|GetWeaponType)))))

(fn IsDoingBehavior
  (params (Behavior :type E_NPCbehavior%20Enum :default "NewEnumerator0"))
  (if (Utilities|Enum|Equal(Enum) Behavior (Variables|Default|GetCurrentBehavior))
    (return false)
    (else
      (Variables|Default|SetCurrentBehavior (Variables|Default|GetBehavior))
      (return true))))

(fn ChangeBehavior
  (params (Enum :type E_NPCbehavior%20Enum :default "NewEnumerator0"))
  (AI|Components|Blackboard|SetValueasEnum (AI|GetBlackboard 0) (Utilities|Name|MakeLiteralName "Behavior") Enum))

(fn AddBehaviorPriority
  (params (NewBehavior :type E_NPCbehavior%20Enum :default "NewEnumerator0"))
  (Utilities|Array|AddUnique (Variables|Default|GetBehaviorPriorities) NewBehavior))

(fn PutOffBehavior
  (params (Priority :type Integer))
  (bind _behaviorpriorities (Variables|Default|GetBehaviorPriorities))
  (bind _behaviorpriorities_2 (Variables|Default|GetBehaviorPriorities))
  (bind _output (Utilities|Array|Get(acopy) _behaviorpriorities))
  (if (> Priority 0)
    (Utilities|Array|Swap _behaviorpriorities_2 0 Priority)
    (CallFunction|ChangeBehavior (Utilities|Array|Get(acopy) _behaviorpriorities_2))
    (else
      (bind _output_get (LocalVariables|SetTempBehavior _output))
      (Utilities|Array|RemoveIndex _behaviorpriorities)
      (Utilities|Array|AddUnique _behaviorpriorities _output_get)
      (CallFunction|ChangeBehavior _output))))