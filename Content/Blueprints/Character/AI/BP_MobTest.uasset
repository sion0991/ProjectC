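; BP_MobTest is a test AI mob on team 2 that sets up a skill, attack range and overhead HP widget on BeginPlay.
; AI perception of a living BP_NPC, or damage from a character, fills an empty blackboard TargetActor and switches the Behavior enum.
; On damage, the attacking character's AttackToTarget applies a test GameplayEffect to the mob, routing hits through GAS.
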(event OnTargetPerceptionUpdated(AIPerception)
  (params (Actor :type Actor%20Object%20Reference) (Stimulus :type AI%20Stimulus%20Structure))
  (bind _returnvalue (AI|GetBlackboard 0))
  (Utilities|IsValid (AI|Components|Blackboard|GetValueasObject (AI|GetBlackboard 0) (Utilities|Name|MakeLiteralName "TargetActor"))
    (:Is%20Not%20Valid
      (bind _asbp_npc (Utilities|Casting|CastToBP_NPC Actor))
      (if (not (Variables|/Script/ProjectC.RPGCharacter|GetIsDeath _asbp_npc))
        (AI|Components|Blackboard|SetValueasObject _returnvalue (Utilities|Name|MakeLiteralName "TargetActor") _asbp_npc)
        (AI|Components|Blackboard|SetValueasEnum _returnvalue (Utilities|Name|MakeLiteralName "Behavior") (Utilities|Enum|LiteralenumE_NPCbehavior "NewEnumerator7"))))))

(event EventBeginPlay
  (CallFunction|InitializeSkill "1001")
  (Variables|Default|SetAttackRange 1.5e+02)
  (|Init3DHPWidget_2)
  (Variables|Default|SetTeamId (Utilities|Struct|MakeGenericTeamId 2)))

(event Game|Damage|EventAnyDamage
  (params (Damage :type Float%20%28single-precision%29) (DamageType :type Damage%20Type%20Object%20Reference) (InstigatedBy :type Controller%20Object%20Reference) (DamageCauser :type Actor%20Object%20Reference))
  (bind _returnvalue (AI|GetBlackboard 0))
  (bind _asbp_character_base (Utilities|Casting|CastToBP_CharacterBase DamageCauser))
  (Class|RPGCharacter|AttacktoTarget _asbp_character_base self "/Game/Blueprints/AbilitySystem/GameplayEffect/BPGE_AttackTest.BPGE_AttackTest_C")
  (Utilities|IsValid (AI|Components|Blackboard|GetValueasObject (AI|GetBlackboard 0) (Utilities|Name|MakeLiteralName "TargetActor"))
    (:Is%20Not%20Valid
      (AI|Components|Blackboard|SetValueasObject _returnvalue (Utilities|Name|MakeLiteralName "TargetActor") _asbp_character_base)
      (AI|Components|Blackboard|SetValueasEnum _returnvalue (Utilities|Name|MakeLiteralName "Behavior") (Utilities|Enum|LiteralenumE_NPCbehavior "NewEnumerator7")))))

(fn ConstructionScript
  (|CallParentFunction))