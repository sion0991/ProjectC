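; BP_CharacterBase is a base character Blueprint in the AI folder that provides shared setup and death handling.
; Init assigns the skeletal mesh and animation class and stores the move and attack ranges.
; The Death event disables capsule collision, pauses mesh animation, switches the mesh to the Death collision profile with physics simulation for a ragdoll-style fall, and sets IsDeath.
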(event EventDeath
  (bind _mesh (Variables|Character|GetMesh))
  (Collision|SetCollisionProfileName (Variables|Default|GetCapsuleComponent) "None" true :!class /Script/Engine.PrimitiveComponent)
  (Variables|/Script/Engine.SkeletalMeshComponent|SetbPauseAnims _mesh true)
  (Collision|SetCollisionProfileName _mesh "Death" true :!class /Script/Engine.PrimitiveComponent)
  (Physics|SetSimulatePhysics _mesh true)
  (Variables|Default|SetIsDeath true))

(fn ConstructionScript)

(fn Init
  (params (SkelMesh :type Skeletal%20Mesh%20Object%20Reference) (AnimClass :type Anim%20Instance%20Class%20Reference) (Move%20Range :type Float%20%28single-precision%29) (Attack%20Range :type Float%20%28single-precision%29))
  (bind _mesh (Variables|Character|GetMesh))
  (Components|SkeletalMesh|SetSkeletalMeshAsset _mesh SkelMesh)
  (Class|SkeletalMeshComponent|SetAnimClass _mesh AnimClass)
  (Variables|Default|SetAttackRange Attack%20Range)
  (Variables|Default|SetMoveRange Move%20Range))