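; BP_AI is an AI Blueprint that sets up combat skills and controls when the AI can act and move.
; InitializeSkill looks up a DT_CharacterData row, then feeds its matching DT_Attack and DT_Finish rows into the ACAttack component.
; ResetAttackCooldown re-enables acting after a short random delay, staggering attack timing.
; SetCanMove writes the movement flag to the Blackboard.
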(event Custom|ResetAttackCooldown
  (Utilities|FlowControl|Delay (Math|Random|RandomFloatinRange 0.5 1.5))
  (Variables|Default|SetIsCanAct true))

(fn ConstructionScript
  (|CallParentFunction))

(fn InitializeSkill
  (params (RowName :type Name))
  (bind _ac_attack (Variables|Default|GetAC_Attack))
  (bind _returnvalue (Utilities|GetDataTableRow "/Game/Blueprints/Data/DT_CharacterData.DT_CharacterData" RowName)
    (:then
      (for _array_element (.attacks _returnvalue)
        (bind _returnvalue_2 (Utilities|GetDataTableRow "/Game/Blueprints/Data/DT_Attack.DT_Attack" _array_element)
          (:then
            (Default|SkillSetting _ac_attack _returnvalue_2))))
      (for _array_element_2 (.finishs _returnvalue)
        (bind _returnvalue_3 (Utilities|GetDataTableRow "/Game/Blueprints/Data/DT_Finish.DT_Finish" _array_element_2)
          (:then
            (Default|SetFinish _ac_attack _returnvalue_3)))))))

(fn SetCanMove
  (params (CanMove :type Boolean))
  (AI|Components|Blackboard|SetValueasBool (AI|GetBlackboard 0) (Utilities|Name|MakeLiteralName "CanMove") CanMove))