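; BP_Skill is a skill Blueprint for C_AI characters, with empty OnSkill and EndSkill functions that appear to be hooks for child skills.
; On BeginPlay it casts its owner to C_AI, stores it as SkillOwner and adds it to the Ignore list.
; IsIgnore loops over that list to report whether a given target is in it, which identifies the skill's own caster.
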(event EventBeginPlay
  (bind _asc_ai (Utilities|Casting|CastToC_AI (Components|GetOwner)))
  (bind _output_get (Variables|Default|SetSkillOwner _asc_ai))
  (Utilities|Array|AddUnique (Variables|Default|GetIgnore) _output_get))

(event Collision|EventActorBeginOverlap
  (params (OtherActor :type Actor%20Object%20Reference)))

(event EventTick
  (params (DeltaSeconds :type Float%20%28single-precision%29)))

(fn ConstructionScript)

(fn OnSkill)

(fn EndSkill)

(fn IsIgnore
  (params (Target :type C%20AI%20Object%20Reference))
  (bind _array_element (Utilities|Array|ForEachLoopwithBreak (Variables|Default|GetIgnore) :!label _label)
    (:LoopBody
      (if (== _array_element Target)
        (goto _label Break)))
    (:Completed
      (return (== _array_element Target)))))