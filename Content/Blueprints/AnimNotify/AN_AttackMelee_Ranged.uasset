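; Anim notify that lands an AI attack on its target when the animation reaches the notify, for mesh owners of type BP_AI.
; It reads the TargetActor character from the AI's blackboard, spawns a scaled-up blood particle at that location and applies Damage credited to the AI's controller.
; The hit goes straight to the blackboard target, with no trace, overlap or range check.
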(fn ReceivedNotify
  (params (MeshComp :type Skeletal%20Mesh%20Component%20Object%20Reference) (Animation :type Anim%20Sequence%20Base%20Object%20Reference) (EventReference :type Anim%20Notify%20Event%20Reference%20Structure%20%28by%20ref%29))
  (bind _asbp_ai (Utilities|Casting|CastToBP_AI (Components|GetOwner MeshComp)))
  (Effects|SpawnEmitteratLocation (.As캐릭터 (Utilities|Casting|CastToCharacter (AI|Components|Blackboard|GetValueasObject (AI|GetBlackboard _asbp_ai) (Utilities|Name|MakeLiteralName "TargetActor")))) "/Game/Effect/P_BloodEffect.P_BloodEffect" (Transformation|GetActorLocation (.As캐릭터 (Utilities|Casting|CastToCharacter (AI|Components|Blackboard|GetValueasObject (AI|GetBlackboard _asbp_ai) (Utilities|Name|MakeLiteralName "TargetActor"))))) "0, 0, 0" "10.000000,10.000000,10.000000")
  (Game|Damage|ApplyDamage (.As캐릭터 (Utilities|Casting|CastToCharacter (AI|Components|Blackboard|GetValueasObject (AI|GetBlackboard _asbp_ai) (Utilities|Name|MakeLiteralName "TargetActor")))) (Variables|Default|GetDamage) (Pawn|GetController _asbp_ai) _asbp_ai (Variables|Default|GetDamage%20Type))
  (return false))