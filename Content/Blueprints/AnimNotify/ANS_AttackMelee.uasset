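; Anim notify state that deals melee damage to opposing-team C_AI during an attack animation window.
; Each tick it sphere-traces between two mesh sockets, with debug drawing on, and compares team IDs on a hit.
; Enemies get a blood effect and ApplyDamage, then join an ignore list that prevents repeat hits until NotifyEnd clears it.
; An AttackToTarget gameplay-effect path exists but is disconnected.
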(fn ReceivedNotifyTick
  (params (MeshComp :type Skeletal%20Mesh%20Component%20Object%20Reference) (Animation :type Anim%20Sequence%20Base%20Object%20Reference) (FrameDeltaTime :type Float%20%28single-precision%29) (EventReference :type Anim%20Notify%20Event%20Reference%20Structure%20%28by%20ref%29))
  (bind _returnvalue (Components|GetOwner MeshComp))
  (bind _as캐릭터 (Utilities|Casting|CastToCharacter _returnvalue))
  (bind _outhit (Collision|SphereTraceForObjects MeshComp (Transformation|GetSocketLocation MeshComp (Variables|Default|GetStart%20Socket)) (Transformation|GetSocketLocation MeshComp (Variables|Default|GetEndSocket)) (Variables|Default|GetRadius) (LocalVariables|GetObjectType) false (Variables|Default|GetActors%20to%20Ignore) "ForDuration" true "(R=1.000000,G=0.000000,B=0.000000,A=1.000000)" "(R=0.000000,G=1.000000,B=0.000000,A=1.000000)" 0.1))
  (if (.bBlockingHit (Collision|BreakHitResult _outhit))
    (if (!= (.teamid (Variables|/Script/ProjectC.RPGCharacter|GetTeamId (.AsC%20AI (Utilities|Casting|CastToC_AI (Components|GetOwner MeshComp))))) (.teamid (Variables|/Script/ProjectC.RPGCharacter|GetTeamId (.AsC%20AI (Utilities|Casting|CastToC_AI (.HitActor (Collision|BreakHitResult _outhit)))))))
      (Utilities|Array|Add (Variables|Default|GetActors%20to%20Ignore) (.HitActor (Collision|BreakHitResult _outhit)))
      (Effects|SpawnEmitteratLocation MeshComp "/Game/Effect/P_BloodEffect.P_BloodEffect" (.Location (Collision|BreakHitResult _outhit)) (Math|Conversions|RotationFromXVector (.ImpactNormal (Collision|BreakHitResult _outhit))) "10.000000,10.000000,10.000000")
      (Game|Damage|ApplyDamage (.HitActor (Collision|BreakHitResult _outhit)) (Variables|Default|GetDamage) (Pawn|GetController _as캐릭터) _as캐릭터 (Variables|Default|GetDamage%20Type))
      (return false))
    (else
      (return false))))

(fn ReceivedNotifyEnd
  (params (MeshComp :type Skeletal%20Mesh%20Component%20Object%20Reference) (Animation :type Anim%20Sequence%20Base%20Object%20Reference) (EventReference :type Anim%20Notify%20Event%20Reference%20Structure%20%28by%20ref%29))
  (Utilities|Array|Clear (Variables|Default|GetActors%20to%20Ignore))
  (return false))

(fn ReceivedNotifyBegin
  (params (MeshComp :type Skeletal%20Mesh%20Component%20Object%20Reference) (Animation :type Anim%20Sequence%20Base%20Object%20Reference) (TotalDuration :type Float%20%28single-precision%29) (EventReference :type Anim%20Notify%20Event%20Reference%20Structure%20%28by%20ref%29))
  (return false))