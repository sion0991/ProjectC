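; Attack component for C_AI characters that manages a list of skills with per-skill cooldowns.
; SkillSetting registers skills alongside a parallel CanUse array, which CoolDown restores after each skill's delay.
; Attacks run by index or by random pick among ready skills (blocked by Stun), playing the montage and storing the active skill class.
; SpawnSkillEffect spawns that class at the owner's transform and calls OnSkill; SetFinish separately collects unique finish data.
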(event Custom|CoolDown
  (params (SkillIndex :type Integer))
  (Utilities|Array|SetArrayElem (Variables|Default|GetCanUse) SkillIndex false)
  (Utilities|FlowControl|Delay (Utilities|Struct|BreakST_Attack (Utilities|Array|Get(acopy) (Variables|Default|GetSkills) SkillIndex)))
  (Utilities|Array|SetArrayElem (Variables|Default|GetCanUse) SkillIndex true))

(event Custom|SkillSetting
  (params (AttackInfo :type ST%20Attack%20Structure))
  (Utilities|Array|AddUnique (Variables|Default|GetSkills) AttackInfo)
  (Utilities|Array|Add (Variables|Default|GetCanUse) true))

(fn SetFinish
  (params (NewItem :type ST%20Finish%20Structure%20%28by%20ref%29))
  (Utilities|Array|AddUnique (Variables|Default|GetFinishData) NewItem))

(fn CanUseAttack
  (params (Index :type Integer))
  (return (Utilities|Array|Get(acopy) (Variables|Default|GetCanUse) Index)))

(fn FindCanUseAttack
  (bind _canuseindex (LocalVariables|GetCanUseIndex))
  (for (_array_element _array_index) (Variables|Default|GetCanUse)
    (if _array_element
      (Utilities|Array|Add (LocalVariables|GetCanUseIndex) _array_index)))
  (if (Utilities|Array|IsValidIndex _canuseindex)
    (bind _output_get (LocalVariables|SetUseIndex (Utilities|Array|Get(acopy) _canuseindex (Math|Random|RandomIntegerinRange 0 (- (Utilities|Array|Length (LocalVariables|GetCanUseIndex)) 1)))))
    (return (Utilities|Array|Get(acopy) (Variables|Default|GetSkills) _output_get) _output_get true)
    (else
      (return "" 0 false))))

(fn SpawnSkillEffect
  (bind _returnvalue (Components|GetOwner))
  (bind _as캐릭터 (Utilities|Casting|CastToCharacter _returnvalue))
  (bind _returnvalue_2 (Game|SpawnActorfromClass (Variables|Default|GetCurrentActiveSkill) (Transformation|GetActorTransform _as캐릭터) "Undefined" "SelectDefaultAtRuntime" _as캐릭터 _as캐릭터))
  (Default|OnSkill _returnvalue_2))

(fn OnAttackAI
  (params (Index :type Integer))
  (bind _skills (Variables|Default|GetSkills))
  (bind _output (Utilities|Array|Get(acopy) _skills Index))
  (bind (_skill _montage) (Utilities|Struct|BreakST_Attack _output))
  (if (CallFunction|CanUseAttack Index)
    (bind _asbp_character_base (Utilities|Casting|CastToC_AI (Components|GetOwner)))
    (Animation|PlayAnimMontage _asbp_character_base _montage 1.0 "None")
    (Variables|Default|SetCurrentActiveSkill _skill)
    (CallFunction|CoolDown Index)))

(fn OnRandomAttack
  (if (Variables|Default|GetStun)
    _
    (else
      (bind (_skill _skillindex _isattack) (CallFunction|FindCanUseAttack))
      (if _isattack
        (bind _asbp_character_base (Utilities|Casting|CastToC_AI (Components|GetOwner)))
        (Animation|PlayAnimMontage _asbp_character_base (.Montage (Utilities|Struct|BreakST_Attack _skill)) 1.0 "None")
        (Variables|Default|SetCurrentActiveSkill (.Skill (Utilities|Struct|BreakST_Attack _skill)))
        (CallFunction|CoolDown _skillindex)
        (return true)
        (else
          _))))
  (return false))